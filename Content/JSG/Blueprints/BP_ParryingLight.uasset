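; BP_ParryingLight is a short-lived light actor, named for parrying, that produces a fading flash and then removes itself.
; On BeginPlay it sets its PointLight to an initial intensity.
; Each Tick subtracts a fixed step from that intensity without delta-time scaling, so the fade speed depends on frame rate.
; Tick also accumulates elapsed time and destroys the actor once the configured lifetime is reached.
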(event `self.ReceiveBeginPlay`
  (`LightComponent.SetIntensity` (`self.PointLight`) (`self.InitLightScale`)))

(event `self.ReceiveTick`
  (params (DeltaSeconds :type "Float (single-precision)"))
  (set `self.CurrentTime` (+ DeltaSeconds (`self.CurrentTime`)))
  (`LightComponent.SetIntensity` (`self.PointLight`) (- (`LightComponentBase.Intensity` (`self.PointLight`)) (`self.DecreaseScale`)))
  (if (>= (`self.CurrentTime`) (`self.DestroyTime`))
    (`self.K2_DestroyActor`)))

(fn `UserConstructionScript`)